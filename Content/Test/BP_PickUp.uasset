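; Ammo pickup actor that the Pacman player collects by walking into it.
; The first box overlap with a Player-tagged actor swaps the mesh to an emissive material and increases BP_Pacman's ammo.
; It also plays a sound and spawns a short-lived noise emitter at the pickup.
; A timeline lerps the mesh toward the first-person camera and toward a target scale, then destroys the actor.
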(event OnComponentBeginOverlap(StaticMesh)
  (params (OverlappedComponent :type Primitive%20Component%20Object%20Reference) (OtherActor :type Actor%20Object%20Reference) (OtherComp :type Primitive%20Component%20Object%20Reference) (OtherBodyIndex :type Integer) (bFromSweep :type Boolean) (SweepResult :type Hit%20Result%20Structure%20%28by%20ref%29)))

(event OnComponentBeginOverlap(Box)
  (params (OverlappedComponent :type Primitive%20Component%20Object%20Reference) (OtherActor :type Actor%20Object%20Reference) (OtherComp :type Primitive%20Component%20Object%20Reference) (OtherBodyIndex :type Integer) (bFromSweep :type Boolean) (SweepResult :type Hit%20Result%20Structure%20%28by%20ref%29))
  (bind _returnvalue (Transformation|GetActorLocation))
  (bind _staticmesh (Variables|Default|GetStaticMesh))
  (if (not (Variables|Default|GetCollidedWithPlayer))
    (if (Actor|ActorHasTag OtherActor "Player")
      (Variables|Default|SetCollidedWithPlayer true)
      (Rendering|Material|SetMaterial (Variables|Default|GetStaticMesh) 0 "/Game/Main/Materials/M_Emissive_Light.M_Emissive_Light")
      (bind _asbp_pacman (Utilities|Casting|CastToBP_Pacman OtherActor))
      (Class|PacManPlayer|IncreaseAmmo _asbp_pacman)
      (Audio|SpawnSoundatLocation 0 _returnvalue "0, 0, 0" 1.0 1.0 0.0 0 0)
      (Class|MyFunctionLib|SpawnNoiseEmitter _returnvalue self 4e+02 3.0 false)
      (bind _newtrack_0 (Timeline|ScalePickup Play)
        (:Update
          (Transformation|SetWorldLocation _staticmesh (Math|Vector|Lerp(Vector) (Transformation|GetActorLocation) (Transformation|GetWorldLocation (Variables|/Script/AITeam12.PlayerCharacter|GetFPSCamera _asbp_pacman)) _newtrack_0) false false)
          (Transformation|SetRelativeTransform _staticmesh (Math|Transform|MakeTransform "0, 0, 0" "0, 0, 0" (.scale (Math|Transform|Lerp(Transform) (Math|Transform|MakeTransform "0, 0, 0" "0, 0, 0" (.scale (Transformation|GetRelativeTransform _staticmesh))) (Math|Transform|MakeTransform "0, 0, 0" "0, 0, 0" (.scale (Variables|Default|GetTransform))) _newtrack_0))) false true))
        (:Finished
          (Actor|DestroyActor))))))

(fn ConstructionScript)