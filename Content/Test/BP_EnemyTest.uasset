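; Test enemy pawn that wanders to random nearby points and reacts to what it sees and hears, driven by Blueprint flags.
; Tick either turns it toward the chased player or starts AI moves while it is idle.
; Vision starts a chase and searches the player's location on loss; hearing sends it to investigate noises unless chasing.
; The health component's damage event only prints the amount.
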(event OnNoiseHeared(HearingComponent)
  (params (HearingInfo :type Hearing%20Info%20Structure%20%28by%20ref%29))
  ;[1 1 1] Hearing
  (if (not (Variables|Default|GetChasing))
    (Variables|Default|SetAlerted true)
    (Transformation|SetActorRotation (Math|Rotator|MakeRotator 0.0 0.0 (.yaw (Math|Rotator|FindLookatRotation (Transformation|GetActorLocation) (.location HearingInfo)))))
    (AI|AIMoveTo (Variables|Default|GetMyAiComponent) self (.location HearingInfo) 0 5.0 false
      (:OnSuccess
        (Utilities|FlowControl|Delay 3.0)
        (Variables|Default|SetAlerted false)
        (Variables|Default|SetMoving false)))))

(event OnTargetSeen(VisionComponent)
  (params (Results :type Vision%20Result%20Structure%20%28by%20ref%29))
  ;[1 1 1] Vision
  (Variables|Default|SetChasing true)
  (Variables|Default|SetPlayer (.seenactor Results))
  (AI|Navigation|MovetoActor (Variables|Default|GetMyAiComponent) (.seenactor Results) -1.0 true true true 0))

(event OnTargetLost(VisionComponent)
  (params (Results :type Vision%20Result%20Structure%20%28by%20ref%29))
  ;[1 1 1] Vision
  (Variables|Default|SetChasing false)
  (Variables|Default|SetAlerted true)
  (AI|AIMoveTo (Variables|Default|GetMyAiComponent) self (Transformation|GetActorLocation (Variables|Default|GetPlayer)) 0 5.0 false
    (:OnSuccess
      (Variables|Default|SetPlayer 0)
      (Variables|Default|SetAlerted false)
      (Variables|Default|SetMoving false))))

(event OnTakeDamage(HealthComponent)
  (params (Damage :type Float%20%28single-precision%29))
  ;[1 1 1] Health/Damage
  (Development|PrintString (Utilities|String|Append "Took Damage " (Utilities|String|ToString(Float) Damage))))

(event EventBeginPlay
  (bind _asaicontroller (Utilities|Casting|CastToAIController (Pawn|GetController)))
  (Variables|Default|SetMyAiComponent _asaicontroller))

(event Collision|EventActorBeginOverlap
  (params (OtherActor :type Actor%20Object%20Reference)))

(event EventTick
  (params (DeltaSeconds :type Float%20%28single-precision%29))
  (bind _returnvalue (Transformation|GetActorLocation))
  ;[1 1 1] Tick/Uppdate
  (if (Variables|Default|GetChasing)
    (Transformation|SetActorRotation (Math|Rotator|MakeRotator 0.0 0.0 (.yaw (Math|Rotator|FindLookatRotation _returnvalue (Transformation|GetActorLocation (Variables|Default|GetPlayer))))))
    (elif (Variables|Default|GetAlerted)
      (Utilities|FlowControl|Delay 2.0 :!label _label)
      (elif (Variables|Default|GetMoving)
        (goto _label)
        (else
          (Variables|Default|SetMoving true)
          (AI|AIMoveTo (Variables|Default|GetMyAiComponent) self (.RandomLocation (AI|Navigation|GetRandomReachablePointinRadius _returnvalue 1e+03 0 0)) 0 5.0 false
            (:OnSuccess
              (Utilities|FlowControl|Delay 2.0)
              (Variables|Default|SetMoving false))))))))

(fn ConstructionScript)