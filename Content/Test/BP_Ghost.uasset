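; BP_Ghost is an enemy ghost that patrols, hunts BP_Pacman and respawns at its start point after death.
; Tick drives flag-based states: patrolling to follow-spline points, returning when far from spawn, facing requested velocity, damaging the player up close and timing respawn.
; Vision starts a chase, or on losing sight sends it to the player's position; hearing sends it to investigate noises.
; Death only hides the actor until respawn restores health.
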(event OnNoiseHeared(HearingComponent)
  (params (HearingInfo :type Hearing%20Info%20Structure%20%28by%20ref%29))
  ;[1 1 1] Hearing
  (if (not (Variables|Default|GetDead))
    (if (not (Variables|Default|GetChasing))
      (Variables|Default|SetAlerted true)
      (Transformation|SetActorRotation (Math|Rotator|MakeRotator 0.0 0.0 (.yaw (Math|Rotator|FindLookatRotation (Transformation|GetActorLocation) (.location HearingInfo)))))
      (AI|AIMoveTo (Variables|Default|GetMyAiComponent) self (.location HearingInfo) 0 5.0 false
        (:OnSuccess
          (Utilities|FlowControl|Delay 3.0)
          (Variables|Default|SetAlerted false)
          (Variables|Default|SetMoving false))))))

(event OnTargetSeen(VisionComponent)
  (params (Results :type Vision%20Result%20Structure%20%28by%20ref%29))
  (bind _asbp_pacman (Utilities|Casting|CastToBP_Pacman (.seenactor Results)))
  ;[1 1 1] Vision
  (if (not (Variables|Default|GetDead))
    (Variables|Default|SetChasing true)
    (Variables|Default|SetPlayer _asbp_pacman)
    (Class|AIEnemy|UpdateTarget _asbp_pacman)
    (AI|Navigation|MovetoActor (Variables|Default|GetMyAiComponent) (.seenactor Results) -1.0 true true true 0)))

(event OnTargetLost(VisionComponent)
  (params (Results :type Vision%20Result%20Structure%20%28by%20ref%29))
  ;[1 1 1] Vision
  (Variables|Default|SetChasing false)
  (Variables|Default|SetAlerted true)
  (AI|AIMoveTo (Variables|Default|GetMyAiComponent) self (Transformation|GetActorLocation (Variables|Default|GetPlayer)) 0 5.0 false
    (:OnSuccess
      (Variables|Default|SetAlerted false)
      (Variables|Default|SetMoving false))))

(event OnTakeDamage(HealthComponent)
  (params (Damage :type Float%20%28single-precision%29))
  ;[1 1 1] Health/Damage
  (Development|PrintString (Utilities|String|Append "Took Damage " (Utilities|String|ToString(Float) Damage))))

(event EventBeginPlay
  (bind _asaicontroller (Utilities|Casting|CastToAIController (Pawn|GetController)))
  (Variables|Default|SetMyAiComponent _asaicontroller)
  ;[1 1 1] Rotation
  (Variables|Default|SetSpawnLocation (Transformation|GetActorLocation)))

(event Collision|EventActorBeginOverlap
  (params (OtherActor :type Actor%20Object%20Reference)))

(event EventTick
  (params (DeltaSeconds :type Float%20%28single-precision%29))
  (bind _returnvalue (Transformation|GetActorLocation))
  (bind _spawnlocation (Variables|Default|GetSpawnLocation))
  (bind _healthcomponent (Variables|Default|GetHealthComponent))
  (if (Variables|Default|GetDead)
    (if (> (Variables|Default|GetDeathTimer) 0.0)
      (Variables|Default|SetDeathTimer (- (Variables|Default|GetDeathTimer) DeltaSeconds))
      (else
        (Variables|Default|SetDead false)
        (Variables|Default|SetDeathTimer 2e+01)
        (Rendering|SetActorHiddenInGame false)
        (Variables|/Script/AITeam12.HealthComponent|SetHealth _healthcomponent (Variables|/Script/AITeam12.HealthComponent|GetMaxHealth _healthcomponent))
        (Transformation|SetActorLocation _spawnlocation false true)))
    (elif (Variables|Default|GetChasing)
      ;[1 1 1] DamagePlayer
      (if (< (Math|Vector|Distance(Vector) (Transformation|GetActorLocation) (Transformation|GetActorLocation (Variables|Default|GetPlayer))) 3.5e+02)
        (Class|AIEnemy|DamagePlayer))
      ;[1 1 1] Rotation
      (Transformation|SetActorRotation (Math|Rotator|MakeRotator 0.0 0.0 (.yaw (Math|Rotator|FindLookatRotation _returnvalue (+ _returnvalue (Variables|/Script/AITeam12.NavMoveComponent|GetRequestedVelocity (Variables|Default|GetNavigationComponent)))))) :!label _label)
      (elif (Variables|Default|GetAlerted)
        (goto _label)
        (else
          ;[1 1 1] Tick/Uppdate
          (if (> (Math|Vector|Distance(Vector) (Transformation|GetActorLocation) _spawnlocation) 8e+03)
            (AI|AIMoveTo (Variables|Default|GetMyAiComponent) self _spawnlocation 0 5.0 false)
            (elif (Variables|Default|GetMoving)
              (goto _label)
              (else
                (Variables|Default|SetMoving true)
                (bind _returnvalue_2 (Class|AIEnemy|GetFollowSplinePoint))
                (AI|AIMoveTo (Variables|Default|GetMyAiComponent) self _returnvalue_2 0 5.0 false
                  (:OnSuccess
                    (Variables|Default|SetMoving false)
                    (Utilities|FlowControl|Delay 3.0)))))))))))

(event EventOnDeath
  ;[1 1 1] Death
  (Variables|Default|SetDead true)
  (Rendering|SetActorHiddenInGame true))

(fn ConstructionScript)