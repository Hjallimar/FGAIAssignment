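; BP_Pacman is a test Pacman player Blueprint with ammo, firing and an overlay widget created at BeginPlay.
; Ammo pickup and fire events update the count text and the plane's emissive color, with a brief orange flash and widget flash on pickup.
; Firing also spawns a noise emitter at the player's location.
; Taking damage teleports the player to the start position, while both win and game over quit the game.
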(event OnTakeDamage(HealthComponent)
  (params (Damage :type Float%20%28single-precision%29))
  (Transformation|SetActorLocation (Variables|Default|GetStartPosition) false true))

(event Custom|CheckAmmo
  (bind _plane (Variables|Default|GetPlane))
  (if (<= (Variables|Default|GetCurrentAmmo) 0)
    (Rendering|Material|SetMaterial _plane 0 "/Game/Main/Materials/M_Emissive_Red.M_Emissive_Red")
    (else
      (Rendering|Material|SetMaterial _plane 0 "/Game/Main/Materials/M_Emissive_Blue.M_Emissive_Blue"))))

(event EventBeginPlay
  (bind _returnvalue (UserInterface|CreateWidget "/Game/Main/Widgets/W_Overlay.W_Overlay_C"))
  (bind _output_get (Variables|Default|SetUI%20Reference _returnvalue))
  (UserInterface|Viewport|AddtoViewport _output_get 0)
  (CallFunction|CheckAmmo))

(event EventPlayerWin
  (Game|QuitGame 0 "Quit" false))

(event EventPlayerGameOver
  (Game|QuitGame 0 "Quit" false))

(event EventAmmoIncrease
  (Default|FlashPickupText (Variables|Default|GetUI%20Reference))
  (Rendering|Components|TextRender|SetText (Variables|Default|GetTextRender) (Utilities|Text|ToText(Integer) (Variables|Default|GetCurrentAmmo) false true 3))
  (Rendering|Material|SetMaterial (Variables|Default|GetPlane) 0 "/Game/Main/Materials/M_Emissive_Orange.M_Emissive_Orange")
  (Utilities|FlowControl|Delay 0.1)
  (CallFunction|CheckAmmo))

(event EventPlayerFire
  (Rendering|Components|TextRender|SetText (Variables|Default|GetTextRender) (Utilities|Text|ToText(Integer) (Variables|Default|GetCurrentAmmo) false true 3))
  (Class|MyFunctionLib|SpawnNoiseEmitter (Transformation|GetActorLocation) self 5e+02 0.5 false)
  (CallFunction|CheckAmmo))

(fn ConstructionScript)